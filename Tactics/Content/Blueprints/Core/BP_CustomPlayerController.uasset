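; BP_CustomPlayerController is a player controller that toggles the game's pause menu with the P key.
; A FlipFlop alternates between pausing with a newly created WBP_PauseMenu that plays PauseFade, and unpausing with focus returned to the viewport and the fade reversed.
; The menu's unpause callback re-enters the same FlipFlop, keeping key and menu toggles in step.
; No explicit widget removal happens here.
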(event `Key|P` :paused true
  (params (Key :type "Key Structure"))
  (:`Pressed`
    (`/Engine/EditorBlueprintResources/StandardMacros.FlipFlop` :!label _label
      (:`A`
        (`GameplayStatics.SetGamePaused` true)
        (bind _returnvalue (`|CreateWidget` "/Game/Blueprints/Widgets/WBP_PauseMenu.WBP_PauseMenu_C" self))
        (add `/Game/Blueprints/Widgets/WBP_PauseMenu.Unpause` _returnvalue (delegate `Unpause`))
        (`UserWidget.AddToViewport` _returnvalue 0)
        (bind _pausefade (`/Game/Blueprints/Widgets/WBP_PauseMenu.PauseFade` _returnvalue))
        (`UserWidget.PlayAnimation` _returnvalue _pausefade 0.0 1 "Forward" 1.0 false))
      (:`B`
        (`GameplayStatics.SetGamePaused` false)
        (`WidgetBlueprintLibrary.SetFocusToGameViewport`)
        (`UserWidget.PlayAnimation` _returnvalue _pausefade 0.0 1 "Reverse" 1.0 false)))))

(event `Unpause`
  (goto _label))

(fn `UserConstructionScript`)